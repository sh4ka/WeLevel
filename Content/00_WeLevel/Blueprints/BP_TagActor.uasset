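; BP_TagActor is an actor that shows gameplay tags from its Ability System component on a text render.
; Each Tick, it reads the owned tags and, if any exist, displays the first one as "Tags: {tag}".
; An Applyeffect event prints a debug message and applies a given Gameplay Effect to itself at level 0.
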(event Custom|Apply%20effect
  (params (Gameplay%20Effect :type Gameplay%20Effect%20Class%20Reference))
  (Development|PrintString "Calling apply effect")
  (GameplayEffects|ApplyGameplayEffectToSelf :self (Variables|Default|GetAbilitySystem) :GameplayEffectClass Gameplay%20Effect))

(event EventBeginPlay)

(event Collision|EventActorBeginOverlap
  (params (OtherActor :type Actor%20Object%20Reference)))

(event EventTick
  (params (DeltaSeconds :type Float%20%28single-precision%29))
  (bind _abilitysystem (Variables|Default|GetAbilitySystem))
  (bind _tagcontainer (GameplayTags|GetOwnedGameplayTags _abilitysystem :!class /Script/GameplayTags.GameplayTagAssetInterface))
  (if (> (Utilities|Array|Length (.gameplaytags _tagcontainer)) 0)
    (Rendering|Components|TextRender|SetText (Variables|Default|GetTextRender) (Utilities|Text|FormatText "Tags: {tag}" (Utilities|Text|ToText(Name) (GameplayTags|GetTagName (Utilities|Array|Get(acopy) (.gameplaytags _tagcontainer))))))))

(fn ConstructionScript)