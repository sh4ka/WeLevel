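; BP_TagActorSphere is a test actor with a sphere mesh that destroys itself in response to a gameplay tag on another actor.
; On BeginPlay it binds to a Destroyed dispatcher, then waits for WeLevel.Test.Tag0 to be added to the first BP_TagActorCube's ability system.
; The added tag fires the dispatcher, and DestroyedEvent removes the sphere and prints a debug message.
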(event Custom|DestroyedEvent
  (Actor|DestroyActor)
  (Development|PrintString "Sphere destroyed event"))

(event EventBeginPlay
  (|CallParentFunction)
  (Utilities|FlowControl|Sequence
    (:then_0
      ;[1 1 1] Bind multicast event
      (EventDispatchers|BindEventtoDestroyed (EventDispatchers|CreateEvent :!event Custom|DestroyedEvent)))
    (:then_1
      (bind _outactors (Actor|GetAllActorsOfClass "/Game/00_WeLevel/Blueprints/BP_TagActorCube.BP_TagActorCube_C"))
      (|WaitforTagAddtoActor (Variables|/Game/00_WeLevel/Blueprints/BP_TagActor.BP_TagActor_C|GetAbilitySystem (Utilities|Array|Get(acopy) _outactors)) "(TagName=\"WeLevel.Test.Tag0\")"
        (:Added
          (Default|CallDestroyed))))))

(fn ConstructionScript
  (|CallParentFunction)
  (Components|StaticMesh|SetStaticMesh (Variables|Default|GetStaticMesh) "/Engine/BasicShapes/Sphere.Sphere"))